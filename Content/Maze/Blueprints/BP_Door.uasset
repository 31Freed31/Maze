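; BP_Door is a maze door actor that swings open when interacted with, once it has been unlocked.
; The Control event opens a Gate node, which lets Interact play the OpenDoor timeline that drives the actor's relative yaw.
; Nothing closes the gate or reverses the timeline, and a few disconnected transform nodes are left unused.
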(event EventBeginPlay
  (|CallParentFunction) ; This node is disabled and will not be called.\nDrag off pins to build functionality.
)

(event Collision|EventActorBeginOverlap
  (params (OtherActor :type Actor%20Object%20Reference))
  (|CallParentFunction OtherActor) ; This node is disabled and will not be called.\nDrag off pins to build functionality.
)

(event EventTick
  (params (DeltaSeconds :type Float%20%28single-precision%29))
  (|CallParentFunction DeltaSeconds) ; This node is disabled and will not be called.\nDrag off pins to build functionality.
)

(event EventInteract
  (Utilities|FlowControl|Gate true
    (:Exit
      (bind _newtrack_4 (Timeline|OpenDoor Play)
        (:Update
          (Transformation|SetActorRelativeRotation (Math|Rotator|MakeRotator 0.0 0.0 _newtrack_4)))))))

(event EventControl
  (Utilities|FlowControl|Gate true) ; enters at Open
)

(fn ConstructionScript
  (|CallParentFunction))