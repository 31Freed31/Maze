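; BP_LiftingGate is a maze gate that alternates between raised and lowered positions when triggered through its Control event.
; Control sets a timer that fires OpenOrClose after a short delay; nothing in this Blueprint calls Control.
; OpenOrClose uses a FlipFlop to offset the actor's Z location up, then back down, snapping instantly without interpolation.
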(event Custom|Open%20or%20Close
  (bind _returnvalue (Transformation|GetActorLocation))
  (bind _returnvalue_2 (Transformation|GetActorLocation))
  (Utilities|FlowControl|FlipFlop
    (:A
      (Transformation|SetActorLocation (Math|Vector|MakeVector (.x _returnvalue_2) (.y _returnvalue_2) (+ (.z _returnvalue_2) 3e+02)) false false))
    (:B
      (Transformation|SetActorLocation (Math|Vector|MakeVector (.x _returnvalue) (.y _returnvalue) (- (.z _returnvalue) 3e+02)) false false))))

(event EventBeginPlay
  (|CallParentFunction) ; This node is disabled and will not be called.\nDrag off pins to build functionality.
)

(event Collision|EventActorBeginOverlap
  (params (OtherActor :type Actor%20Object%20Reference))
  (|CallParentFunction OtherActor) ; This node is disabled and will not be called.\nDrag off pins to build functionality.
)

(event EventTick
  (params (DeltaSeconds :type Float%20%28single-precision%29))
  (|CallParentFunction DeltaSeconds) ; This node is disabled and will not be called.\nDrag off pins to build functionality.
)

(event EventControl
  (Utilities|Time|SetTimerbyEvent (delegate Custom|Open%20or%20Close) 3.0))

(fn ConstructionScript
  (|CallParentFunction))