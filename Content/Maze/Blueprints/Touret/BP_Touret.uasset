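; Maze turret that sweeps back and forth on a timeline and shoots the player character when spotted.
; Tick runs a Patrol/Shoot state machine: a forward sphere trace detects the player, then the turret turns its yaw toward them.
; A looping timer fires line-trace shots with sound and particles, applying a damage GameplayEffect on hit.
; Losing the trace clears the timer and resumes patrol from the current rotation.
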(event Custom|StartPatrol
  (bind _rotatetrack (Timeline|Timeline PlayFromStart)
    (:Update
      (Transformation|SetWorldRotation (Variables|Default|GetSkeletalMesh) (Math|Rotator|Lerp(Rotator) (Variables|Default|GetCurrentRotation) (Variables|Default|GetTargetRotation) _rotatetrack) false false))
    (:Finished
      (switch Utilities|FlowControl|Switch|SwitchonETimelineDirection (Variables|Default|GetDirectionMove)
        (:Forward
          (Variables|Default|SetDirectionMove "Backward")
          (Variables|Default|SetTargetRotation (Variables|Default|GetStartRotation))
          (Variables|Default|SetCurrentRotation (Variables|Default|GetEndRotation)))
        (:Backward
          (Variables|Default|SetDirectionMove "Forward")
          (Variables|Default|SetTargetRotation (Variables|Default|GetEndRotation))
          (Variables|Default|SetCurrentRotation (Variables|Default|GetStartRotation))))
      (CallFunction|StartPatrol))))

(event Custom|StopPatrol
  (bind _rotatetrack (Timeline|Timeline Stop)
    (:Update
      (Transformation|SetWorldRotation (Variables|Default|GetSkeletalMesh) (Math|Rotator|Lerp(Rotator) (Variables|Default|GetCurrentRotation) (Variables|Default|GetTargetRotation) _rotatetrack) false false))
    (:Finished
      (switch Utilities|FlowControl|Switch|SwitchonETimelineDirection (Variables|Default|GetDirectionMove)
        (:Forward
          (Variables|Default|SetDirectionMove "Backward")
          (Variables|Default|SetTargetRotation (Variables|Default|GetStartRotation))
          (Variables|Default|SetCurrentRotation (Variables|Default|GetEndRotation)))
        (:Backward
          (Variables|Default|SetDirectionMove "Forward")
          (Variables|Default|SetTargetRotation (Variables|Default|GetEndRotation))
          (Variables|Default|SetCurrentRotation (Variables|Default|GetStartRotation))))
      (CallFunction|StartPatrol))))

(event Custom|StartShoot
  (bind _returnvalue (Utilities|Time|SetTimerbyEvent (delegate Custom|CallShootFunc) 1.0 true))
  (Variables|Default|SetShootTimer _returnvalue))

(event Custom|CallShootFunc
  (bind _isshoot (CallFunction|Shoot))
  (if _isshoot
    (bind _asbp_base_player_character (Utilities|Casting|CastToBP_BasePlayerCharacter (Game|GetPlayerCharacter 0)))
    (GameplayEffects|ApplyGameplayEffectToTarget :self (Variables|Default|GetAbilitySystem) :GameplayEffectClass "/Game/Maze/Core/GameSystem/GameplayAbilities/Touret/GE_TouretDamage.GE_TouretDamage_C" :Target (Variables|/Game/Maze/Core/Characterts/BP_BaseCharacter.BP_BaseCharacter_C|GetAbilitySystem _asbp_base_player_character))))

(event EventTick
  (params (DeltaSeconds :type Float%20%28single-precision%29))
  (bind _skeletalmesh (Variables|Default|GetSkeletalMesh))
  (bind _returnvalue (Transformation|GetWorldRotation _skeletalmesh))
  (Utilities|IsValid (Game|Player|GetPlayerPawn 0)
    (:Is%20Valid
      (switch Utilities|FlowControl|Switch|SwitchonE_TouretStates (Variables|Default|GetCurrentState)
        (:NewEnumerator0
          (bind _isplayerfind (CallFunction|PLayerSearch))
          (if _isplayerfind
            (CallFunction|StopPatrol)
            (Variables|Default|SetCurrentState "NewEnumerator1")))
        (:NewEnumerator1
          (Transformation|SetWorldRotation _skeletalmesh (Math|Interpolation|RInterpTo (Math|Rotator|MakeRotator (.roll _returnvalue) (.pitch _returnvalue) (.yaw _returnvalue)) (Math|Rotator|MakeRotator (.roll _returnvalue) (.pitch _returnvalue) (- (.yaw (Math|Rotator|FindLookatRotation (Transformation|GetWorldLocation (Variables|Default|GetSkeletalMesh)) (Transformation|GetActorLocation (Game|GetPlayerCharacter 0)))) 9e+01)) (Utilities|Time|GetWorldDeltaSeconds) 0.0) false false)
          (Utilities|FlowControl|Sequence
            (:then_0
              (if (not (Variables|Default|GetIsStartShootl))
                (CallFunction|StartShoot)
                (Variables|Default|SetIsStartShootl true)))
            (:then_1
              (bind _isplayerfind_2 (CallFunction|PLayerSearch))
              (if (not _isplayerfind_2)
                (Utilities|Time|ClearandInvalidateTimerbyHandle (Variables|Default|GetShootTimer))
                (Variables|Default|SetIsStartShootl false)
                (Variables|Default|SetCurrentState "NewEnumerator0")
                (Variables|Default|SetTargetRotation (Variables|Default|GetEndRotation))
                (Variables|Default|SetCurrentRotation (Transformation|GetWorldRotation (Variables|Default|GetSkeletalMesh)))
                (Variables|Default|SetDirectionMove "Forward")
                (CallFunction|StartPatrol)))))))))

(event EventBeginPlay
  (bind _output_get (Variables|Default|SetStartRotation (Transformation|GetWorldRotation (Variables|Default|GetSkeletalMesh))))
  (Variables|Default|SetEndRotation (Math|Rotator|MakeRotator (.roll _output_get) (.pitch _output_get) (+ (.yaw _output_get) 95.0)))
  (Variables|Default|SetCurrentRotation (Variables|Default|GetStartRotation))
  (Variables|Default|SetTargetRotation (Variables|Default|GetEndRotation))
  (CallFunction|StartPatrol))

(fn ConstructionScript)

(fn PLayerSearch
  (bind _scene (Variables|Default|GetScene))
  (bind _returnvalue (Transformation|GetWorldLocation _scene))
  (bind (_outhit _returnvalue_2) (Collision|SphereTraceByChannel _returnvalue (+ _returnvalue (* (Math|Vector|GetForwardVector _scene) (Variables|Default|GetSearchDistance))) 1e+01 "TraceTypeQuery2" false 0 "ForOneFrame" false))
  (if _returnvalue_2
    (Utilities|Casting|CastToBP_BasePlayerCharacter (.HitActor (Collision|BreakHitResult _outhit))
      (:then
        (return true))
      (:CastFailed
        (return false)))
    (else
      (return false))))

(fn Shoot
  (bind _scene (Variables|Default|GetScene))
  (bind _returnvalue (Transformation|GetWorldLocation _scene))
  (bind (_outhit _returnvalue_2) (Collision|LineTraceByChannel _returnvalue (+ _returnvalue (* (Math|Vector|GetForwardVector _scene) (Variables|Default|GetShootDistance))) "TraceTypeQuery2" false 0 "ForOneFrame"))
  (Utilities|FlowControl|Sequence
    (:then_0
      (Audio|PlaySoundatLocation "/Game/Packs/StarterContent/Audio/Explosion01.Explosion01" (Transformation|GetWorldLocation (Variables|Default|GetScene)) "0, 0, 0" 0.05 1.0 0.0 0 0 0 0)
      (Effects|SpawnEmitterAttached "/Game/Packs/StarterContent/Particles/P_Explosion.P_Explosion" (Variables|Default|GetScene) "None"))
    (:then_1
      (if _returnvalue_2
        (Utilities|Casting|CastToBP_BasePlayerCharacter (.HitActor (Collision|BreakHitResult _outhit))
          (:then
            (bind _returnvalue_3 (Effects|SpawnEmitteratLocation "/Game/Packs/FXVarietyPack/Particles/P_ky_hit1.P_ky_hit1" (.Location (Collision|BreakHitResult _outhit)) "0, 0, 0" "0.300000,0.300000,0.300000" true "None" false))
            (Effects|Components|ParticleSystem|SetVectorParameter _returnvalue_3 "color" (Math|Conversions|ToVector(LinearColor) (.SpecifiedColor (Utilities|Struct|BreakSlateColor (Variables|Default|GetColor)))))
            (Components|Activation|Activate _returnvalue_3 false)
            (return true))
          (:CastFailed
            (return false)))
        (else
          (return false))))))