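; Patrol path actor that turns a patrolling character to face the direction of its Arrow component.
; OnPatrollerEntered stores the character and opens a gate on Tick, and OnPatrollerExit closes it.
; While the gate is open, Tick smoothly interpolates the character's rotation toward the arrow's world rotation.
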(event Custom|OnPatrollerEntered
  (params (Character :type Character%20Object%20Reference))
  (bind _output_get (Variables|Default|SetCharacter Character))
  (Utilities|IsValid _output_get
    (:Is%20Valid
      (Utilities|FlowControl|Gate true) ; enters at Open
    )))

(event Custom|OnPatrollerExit
  (bind _character (Variables|Default|GetCharacter))
  (bind _character_2 (Variables|Default|GetCharacter))
  (Utilities|FlowControl|Gate true) ; enters at Close
)

(event EventBeginPlay)

(event EventTick
  (params (DeltaSeconds :type Float%20%28single-precision%29))
  (bind _character (Variables|Default|GetCharacter))
  (bind _character_2 (Variables|Default|GetCharacter))
  (Utilities|FlowControl|Gate true
    (:Exit
      (Utilities|IsValid _character_2
        (:Is%20Valid
          (Utilities|IsValid _character
            (:Is%20Valid
              (Transformation|SetActorRotation _character (Math|Interpolation|RInterpTo (Transformation|GetActorRotation _character_2) (Transformation|GetWorldRotation (Variables|Default|GetArrow)) DeltaSeconds 2.0)))))))))

(fn ConstructionScript)