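; Base character Blueprint for the Maze game, built on the Gameplay Ability System with an overhead health bar widget.
; An async attribute listener calls OnDeath at zero health, applying GE_Death and calling a death dispatcher, while AnyDamage feeds BPHealth.
; Melee collision overlaps with other base characters are confirmed by line trace, then sent to itself as hit gameplay events.
; Helper functions toggle ragdoll and set up physical animation.
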(event OnComponentBeginOverlap(MeleeHitCollision)
  (params (OverlappedComponent :type Primitive%20Component%20Object%20Reference) (OtherActor :type Actor%20Object%20Reference) (OtherComp :type Primitive%20Component%20Object%20Reference) (OtherBodyIndex :type Integer) (bFromSweep :type Boolean) (SweepResult :type Hit%20Result%20Structure%20%28by%20ref%29))
  (if (!= OtherActor self)
    (bind _asbp_base_character (Utilities|Casting|CastToBP_BaseCharacter OtherActor))
    (bind _outhits (Class|KismetSystemLibrary|LineTraceMultiforObjects (Transformation|GetWorldLocation (Variables|Default|GetMeleeHitCollision)) (Transformation|GetActorLocation _asbp_base_character) (Utilities|Array|MakeArray "ObjectTypeQuery3" "ObjectTypeQuery2") false (Utilities|Array|MakeArray self) "None" true))
    (bind _array_element (Utilities|Array|ForEachLoopwithBreak _outhits :!label _label)
      (:LoopBody
        (if (== (.HitActor (Collision|BreakHitResult _array_element)) _asbp_base_character)
          (Ability|SendGameplayEventtoActor self "(TagName=\"Event.Ability.MeleeAttack.Hit\")" (Utilities|Struct|MakeGameplayEventData "(TagName=\"\")" 0 0 0 0 "()" "(GameplayTags=)" "(GameplayTags=)" 0.0 (Ability|TargetData|AbilityTargetDatafromHitResult _array_element)))
          (goto _label Break))))))

(event Custom|OnDeath
  (Utilities|IsValid self
    (:Is%20Valid
      (GameplayEffects|ApplyGameplayEffectToSelf :self (Variables|Default|GetAbilitySystem) :GameplayEffectClass "/Game/Maze/Core/GameSystem/GameplayAbilities/PassiveEffects/GE_Death.GE_Death_C")
      (Default|CallOnDeathDispatcher self))))

(event Game|Damage|EventAnyDamage
  (params (Damage :type Float%20%28single-precision%29) (DamageType :type Damage%20Type%20Object%20Reference) (InstigatedBy :type Controller%20Object%20Reference) (DamageCauser :type Actor%20Object%20Reference))
  (Default|DecreaseHealth (Variables|Default|GetBP_Health) Damage))

(event EventBeginPlay
  (Utilities|FlowControl|Sequence
    (:then_0
      (|CallParentFunction)
      (bind _aswbp_character_health_bar (Utilities|Casting|CastToWBP_CharacterHealthBar (UserInterface|GetWidget (Variables|Default|GetWidget))))
      (Variables|/Game/Maze/Core/UI/WBP_CharacterHealthBar.WBP_CharacterHealthBar_C|SetWidgetOwner _aswbp_character_health_bar self))
    (:then_1
      (bind (_asynctaskproxy _attribute _newvalue _oldvalue) (Ability|Tasks|WaitForAttributeChanged 0 "(AttributeName=\"Health\",Attribute=/Script/Maze.MazeAttributeSet:Health,AttributeOwner=\"/Script/CoreUObject.Class'/Script/Maze.MazeAttributeSet'\")")
        (:Changed
          (Development|PrintText (Utilities|Text|FormatText "HP changed {1}. Old: {2}. New: {3}" self _newvalue _oldvalue))
          (if (<= _newvalue 0.0)
            (Development|PrintText (Utilities|Text|FormatText "{1} is now dead" self))
            (AsyncAction|Cancel _asynctaskproxy)
            (CallFunction|OnDeath)))))))

(fn ConstructionScript)

(fn EnableRagdoll
  (params (InBoneName :type Name))
  (bind _mesh (Variables|Character|GetMesh))
  (Utilities|IsValid _mesh
    (:Is%20Valid
      (LocalVariables|SetInitialTransform (Transformation|GetRelativeTransform _mesh))
      (Collision|SetCollisionProfileName (Variables|Character|GetMesh) "Ragdoll" true :!class /Script/Engine.PrimitiveComponent)
      (Class|SkeletalMeshComponent|SetAllBodiesBelowSimulatePhysics (Variables|Character|GetMesh) InBoneName true true)
      (Variables|Default|SetIsRagdollEnabled true)
      (Pawn|Components|CharacterMovement|DisableMovement (Variables|Character|GetCharacterMovement))
      (return (LocalVariables|GetInitialTransform)))))

(fn DisableRagdoll
  (params (SnapTransform :type Transform%20%28by%20ref%29))
  (Physics|SetSimulatePhysics (Variables|Character|GetMesh) false)
  (Collision|SetCollisionProfileName (Variables|Character|GetMesh) "CharacterMesh" true :!class /Script/Engine.PrimitiveComponent)
  (Transformation|AttachComponentToComponent (Variables|Character|GetMesh) (Variables|Collision|GetCapsuleComponent) "None" "KeepRelative" "KeepRelative" "KeepRelative" true)
  (Transformation|SetRelativeTransform (Variables|Character|GetMesh) SnapTransform false false)
  (Pawn|Components|CharacterMovement|SetMovementMode (Variables|Character|GetCharacterMovement) "MOVE_Walking" 0)
  (Variables|Default|SetIsRagdollEnabled false))

(fn EnablePA
  (params (BodyName :type Name))
  (Class|PhysicalAnimationComponent|SetSkeletalMeshComponent (Variables|Default|GetPhysicalAnimation) (Variables|Character|GetMesh))
  (Class|PhysicalAnimationComponent|ApplyPhysicalAnimationSettingsBelow (Variables|Default|GetPhysicalAnimation) BodyName (Utilities|Struct|MakePhysicalAnimationData false 1e+03 1e+02 1e+03 1e+02) true)
  (Class|SkeletalMeshComponent|SetAllBodiesBelowSimulatePhysics (Variables|Character|GetMesh) BodyName false true)
  (Collision|SetCollisionProfileName (Variables|Character|GetMesh) "Ragdoll" true :!class /Script/Engine.PrimitiveComponent))

(fn DisablePA
  (Class|PhysicalAnimationComponent|SetSkeletalMeshComponent (Variables|Default|GetPhysicalAnimation) (Variables|Character|GetMesh)))