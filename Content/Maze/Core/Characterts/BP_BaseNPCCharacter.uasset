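; BP_BaseNPCCharacter is a base NPC character Blueprint that handles death on top of its parent class's logic.
; On death, if controlled by AI_NPC, it stops the brain logic, ragdolls the body and disables capsule collision and overlaps.
; It then calls RegisterKill on every BP_Kill_NPC actor.
; The one-second delayed self-destroy sits inside that loop, so it runs only when such an actor exists.
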(event EventOnDeath
  (|CallParentFunction)
  (bind _asai_npc (Utilities|Casting|CastToAI_NPC (Pawn|GetController)))
  (AI|Logic|StopLogic (Variables|/Script/AIModule.AIController|GetBrainComponent _asai_npc) "Dead")
  (CallFunction|EnableRagdoll (Variables|Default|GetRootRagdollBone))
  (Collision|SetCollisionEnabled (Variables|Default|GetCapsuleComponent) "NoCollision")
  (Variables|/Script/Engine.PrimitiveComponent|SetbGenerateOverlapEvents (Variables|Default|GetCapsuleComponent) false)
  (bind _outactors (Actor|GetAllActorsOfClass "/Game/Maze/Core/GameSystem/Quests/BP_Kill_NPC.BP_Kill_NPC_C"))
  (bind _output_get (Variables|Default|SetOut%20Actors _outactors))
  (for _array_element _output_get
    (Default|RegisterKill _array_element)
    (Utilities|FlowControl|Delay 1.0)
    (Actor|DestroyActor)))

(fn ConstructionScript
  (|CallParentFunction))

(fn DisablePA
  (|CallParentFunction))