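; Player character Blueprint for Elf Arden, a child class that builds on parent logic for ragdoll, physical animation and melee hit collision.
; Construction snaps the melee hit collision to the right-hand socket, and BeginPlay enables physical animation from a configured bone.
; While ragdolled, Tick sweeps the actor to the mesh's world location so it follows the body.
; The ragdoll and physical animation overrides only forward to the parent.
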(event EventBeginPlay
  (|CallParentFunction)
  (CallFunction|EnablePA (Variables|Default|GetPhysicalAnimationBone_0)))

(event EventTick
  (params (DeltaSeconds :type Float%20%28single-precision%29))
  (|CallParentFunction DeltaSeconds)
  (if (Variables|Default|GetIsRagdollEnabled)
    (Transformation|SetActorLocation (Transformation|GetWorldLocation (Variables|Character|GetMesh)) true false)))

(fn ConstructionScript
  (|CallParentFunction)
  (Transformation|AttachComponentToComponent (Variables|Default|GetMeleeHitCollision) (Variables|Character|GetMesh) "hand_r_socket" "SnapToTarget" "SnapToTarget" "KeepRelative" true))

(fn EnableRagdoll
  (params (InBoneName :type Name :default "None"))
  (bind _initialrelativetransform (|CallParentFunction InBoneName))
  (return _initialrelativetransform))

(fn DisableRagdoll
  (params (SnapTransform :type Transform%20%28by%20ref%29))
  (|CallParentFunction SnapTransform)
  (return))

(fn DisablePA
  (|CallParentFunction))

(fn EnablePA
  (params (BodyName :type Name :default "None"))
  (|CallParentFunction BodyName))