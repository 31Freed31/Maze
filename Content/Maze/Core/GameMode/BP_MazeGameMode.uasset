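; Maze game mode that runs the level time limit, progression, end screens and player respawning.
; A timer started at BeginPlay shows the time-out screen, while WIn opens the next map in Levels or shows the win screen.
; Lose shows its own screen; all end screens pause the game.
; Player death, caught through the character's death dispatcher, triggers a delayed respawn, then resets AI_NPC blackboard values and restarts their brain logic.
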(event Custom|Lose
  (bind _returnvalue (Game|GetPlayerController 0))
  (bind _returnvalue_2 (UserInterface|CreateWidget "/Game/Maze/Core/UI/BP_LOSE.BP_LOSE_C"))
  (UserInterface|Viewport|AddtoViewport _returnvalue_2 0)
  (Input|SetInputModeUIOnly _returnvalue 0 "DoNotLock" false)
  (Variables|/Script/Engine.PlayerController|SetbShowMouseCursor _returnvalue true)
  (Game|SetGamePaused true))

(event Custom|WIn
  (bind _returnvalue (Game|GetPlayerController 0))
  (bind _returnvalue_2 (Game|GetCurrentLevelName true))
  (if (>= (Utilities|Array|FindItem (Variables|Default|GetLevels) (Utilities|String|StringToName _returnvalue_2)) 0)
    (if (< (+ (Utilities|Array|FindItem (Variables|Default|GetLevels) (Utilities|String|StringToName _returnvalue_2)) 1) (Utilities|Array|Length (Variables|Default|GetLevels)))
      (Game|OpenLevel(byName) (Utilities|Array|Get(acopy) (Variables|Default|GetLevels) (+ (Utilities|Array|FindItem (Variables|Default|GetLevels) (Utilities|String|StringToName _returnvalue_2)) 1)))
      (else
        (bind _returnvalue_3 (UserInterface|CreateWidget "/Game/Maze/Core/UI/BP_WIN.BP_WIN_C" :!label _label))
        (UserInterface|Viewport|AddtoViewport _returnvalue_3 0)
        (Input|SetInputModeUIOnly _returnvalue 0 "DoNotLock" false)
        (Variables|/Script/Engine.PlayerController|SetbShowMouseCursor _returnvalue true)
        (Game|SetGamePaused true)))
    (else
      (goto _label))))

(event Custom|OnplayerDeath
  (params (Source :type BP%20Base%20Character%20Object%20Reference))
  (bind _returnvalue (Utilities|Name|MakeLiteralName "AcceptanceRadius"))
  (bind _returnvalue_2 (Game|GetPlayerController 0))
  (bind _currentplayercharacter (Variables|Default|GetCurrentPlayerCharacter))
  (Utilities|IsValid _currentplayercharacter
    (:Is%20Valid
      (EventDispatchers|UnbindEventfromOnDeathDispatcher _currentplayercharacter (delegate Custom|OnplayerDeath))
      (Pawn|UnPossess (Game|GetPlayerController 0))
      (Utilities|FlowControl|Delay 2.0)
      (Class|GameModeBase|RestartPlayer _returnvalue_2)
      (bind _outactors (Actor|GetAllActorsOfClass "/Game/Maze/Core/Characterts/AI/AI_NPC.AI_NPC_C"))
      (for _array_element _outactors
        (bind _asai_npc (Utilities|Casting|CastToAI_NPC _array_element))
        (AI|Components|Blackboard|ClearValue (Variables|/Script/AIModule.AIController|GetBlackboard _asai_npc) _returnvalue)
        (AI|Components|Blackboard|SetValueasObject (Variables|/Script/AIModule.AIController|GetBlackboard _asai_npc) _returnvalue _returnvalue_2)
        (AI|Logic|StopLogic (Variables|/Script/AIModule.AIController|GetBrainComponent _asai_npc) "Restart")
        (AI|Logic|StartLogic (Variables|/Script/AIModule.AIController|GetBrainComponent _asai_npc))))))

(event Custom|Time%20out
  (CallFunction|EndTimer))

(event Custom|EndTimer
  (bind _returnvalue (Game|GetPlayerController 0))
  (bind _returnvalue_2 (UserInterface|CreateWidget "/Game/Maze/Core/UI/BP_LoseTimer.BP_LoseTimer_C"))
  (UserInterface|Viewport|AddtoViewport _returnvalue_2 0)
  (Input|SetInputModeUIOnly _returnvalue 0 "DoNotLock" false)
  (Variables|/Script/Engine.PlayerController|SetbShowMouseCursor _returnvalue true)
  (Game|SetGamePaused true))

(event EventBeginPlay
  (bind _returnvalue (Utilities|Time|SetTimerbyEvent (delegate Custom|Time%20out) (Variables|Default|GetGameTime)))
  (Variables|Default|SetLoseTimer _returnvalue))

(event EventOnRestartPlayer
  (params (NewPlayer :type Controller%20Object%20Reference))
  (bind _asbp_base_character (Utilities|Casting|CastToBP_BaseCharacter (Pawn|GetControlledPawn NewPlayer)))
  (Utilities|IsValid _asbp_base_character
    (:Is%20Valid
      (bind _output_get (Variables|Default|SetCurrentPlayerCharacter _asbp_base_character))
      (EventDispatchers|BindEventtoOnDeathDispatcher _output_get (delegate Custom|OnplayerDeath)))))

(fn ConstructionScript)