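; GA_Sprint is a Gameplay Ability that lets a BP_BaseCharacter avatar sprint while the input is held.
; After committing, it waits for input release while a looping WaitDelay re-commits the cost every tenth of a second, raising MaxWalkSpeed on each success.
; Input release or an unpaid cost sets the slower walk speed and ends the ability.
; OnEndAbility is empty, so other endings do not reset speed.
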(event Ability|EventActivateAbility
  (bind _asbp_base_character (Utilities|Casting|CastToBP_BaseCharacter (Ability|GetAvatarActorfromActorInfo))
    (:then
      (Variables|Default|SetAvatar%20Character _asbp_base_character)
      (bind _returnvalue (Ability|CommitAbility))
      (if _returnvalue
        (Ability|Tasks|WaitInputRelease false
          (:then
            (Ability|Tasks|WaitDelay 0.1 :!label _label
              (:OnFinish
                (bind _returnvalue_2 (Ability|CommitAbilityCost false))
                (if _returnvalue_2
                  (Variables|/Script/Engine.CharacterMovementComponent|SetMaxWalkSpeed (Variables|/Script/Engine.Character|GetCharacterMovement (Variables|Default|GetAvatar%20Character)) 5e+02)
                  (goto _label)
                  (else
                    _)))))
          (:OnRelease
            _))
        (Variables|/Script/Engine.CharacterMovementComponent|SetMaxWalkSpeed (Variables|/Script/Engine.Character|GetCharacterMovement (Variables|Default|GetAvatar%20Character)) 2.5e+02)
        (Ability|EndAbility)
        (else
          (Ability|CancelAbility))))
    (:CastFailed
      (Ability|CancelAbility))))

(event Ability|EventOnEndAbility
  (params (bWasCancelled :type Boolean)))