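; GA_Stealth is a hold-to-use Gameplay Ability that puts the avatar character into stealth.
; On activation it crouches the BP_BaseCharacter avatar, applies GE_Stealth and stores the effect handle, cancelling if the avatar is invalid or another class.
; Releasing input ends the ability, which uncrouches the character and removes the effect by handle.
; This cleanup is skipped when the ability is cancelled.
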(event Ability|EventActivateAbility
  (bind _returnvalue (Ability|GetAvatarActorfromActorInfo))
  (Utilities|IsValid _returnvalue
    (:Is%20Valid
      (bind _asbp_base_character (Utilities|Casting|CastToBP_BaseCharacter _returnvalue)
        (:then
          (bind _output_get (Variables|Default|SetAvatar%20Character _asbp_base_character))
          (Character|Crouch _output_get)
          (bind _returnvalue_2 (Ability|ApplyGameplayEffectToOwner "/Game/Maze/Core/GameSystem/GameplayAbilities/Stealth/GE_Stealth.GE_Stealth_C"))
          (Variables|Default|SetApplied%20Effect _returnvalue_2)
          (Ability|Tasks|WaitInputRelease false
            (:OnRelease
              (Ability|EndAbility))))
        (:CastFailed
          (Ability|CancelAbility))))
    (:Is%20Not%20Valid
      (Ability|CancelAbility))))

(event Ability|EventOnEndAbility
  (params (bWasCancelled :type Boolean))
  (if (not bWasCancelled)
    (Character|UnCrouch (Variables|Default|GetAvatar%20Character))
    (Ability|RemoveGameplayEffectFromOwnerWithHandle (Variables|Default|GetApplied%20Effect))))