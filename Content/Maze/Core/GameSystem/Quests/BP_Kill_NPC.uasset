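; BP_Kill_NPC is a quest Blueprint that tracks a kill objective.
; Each RegisterKill event increments KillsSoFar and sets the quest as completed once the count reaches NeedKills.
; BeginPlay and the construction script only call their parent versions.
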(event Custom|RegisterKill
  (Variables|Default|SetKillsSoFar (+ (Variables|Default|GetKillsSoFar) 1))
  (if (>= (Variables|Default|GetKillsSoFar) (Variables|Default|GetNeedKills))
    (CallFunction|SetIsCompleted true)))

(event EventBeginPlay
  (|CallParentFunction))

(fn ConstructionScript
  (|CallParentFunction))