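; BP_Quest is a quest object for the Maze game that tracks a quest's number, name, active state and completion state.
; Getter and setter functions wrap each field, and the ActivateQuest event marks the quest active through SetIsActive.
; SetIsCompleted fires the OnQuestCompleted dispatcher with the quest itself only when completion changes from false to true, then stores the new value.
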(event Custom|ActivateQuest
  (CallFunction|SetIsActive true))

(fn ConstructionScript)

(fn SetIsCompleted
  (params (NewIsCompleted :type Boolean))
  (if (and NewIsCompleted (not (Variables|Default|GetIsCompleted)))
    (Default|CallOnQuestCompleted self))
  (Variables|Default|SetIsCompleted NewIsCompleted))

(fn GetIsCompleted
  (return (Variables|Default|GetIsCompleted)))

(fn SetQuestNumber
  (params (QuestNumber :type Integer))
  (Variables|Default|SetQuestNumber QuestNumber))

(fn GetQuestNumber
  (return (Variables|Default|GetQuestNumber)))

(fn SetQuestName
  (params (QuestName :type Text))
  (Variables|Default|SetQuestName QuestName))

(fn GetQuestName
  (return (Variables|Default|GetQuestName)))

(fn SetIsActive
  (params (NewIsActive :type Boolean))
  (Variables|Default|SetIsActive NewIsActive))

(fn GetIsActive
  (return (Variables|Default|GetIsActive)))