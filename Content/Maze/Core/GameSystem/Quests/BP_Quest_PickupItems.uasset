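; Quest Blueprint that completes once the player has picked up every tagged pickup item in the level.
; On activation it finds all BP_Pickup actors with the quest's ItemTag, stores their count as the target, activates each one and binds to its OnPickUp event.
; Each pickup increments a counter, and the quest marks itself completed when the counter equals that target.
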(event Custom|OnItemPickedUp
  (Math|Integer|IncrementInt (Variables|Default|GetPickedUpCount)
    (:%20%20
      (if (== (Variables|Default|GetNumberOfitemsToPickUp) (Variables|Default|GetPickedUpCount))
        (CallFunction|SetIsCompleted true)))))

(event EventActivateQuest
  (|CallParentFunction)
  (bind _outactors (Actor|GetAllActorsOfClasswithTag "/Game/Maze/Core/GameSystem/Quests/BP_Pickup.BP_Pickup_C" (Variables|Default|GetItemTag)))
  (Variables|Default|SetNumberOfitemsToPickUp (Utilities|Array|Length _outactors))
  (for _array_element _outactors
    (Default|Activate _array_element)
    (EventDispatchers|BindEventtoOnPickUp _array_element (delegate Custom|OnItemPickedUp))))

(fn ConstructionScript
  (|CallParentFunction))