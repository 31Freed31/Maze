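; BP_Quest_ReachDestination is a quest actor that completes when the current player character reaches its Box trigger volume.
; It extends a parent quest class, keeping the Box overlap events and Cube visual off while inactive and enabling both in ActivateQuest.
; An overlap from a BP_BaseCharacter carrying the exact CurrentPlayer gameplay tag sets the quest completed, then disables the trigger and hides the Cube.
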(event OnComponentBeginOverlap(Box)
  (params (OverlappedComponent :type Primitive%20Component%20Object%20Reference) (OtherActor :type Actor%20Object%20Reference) (OtherComp :type Primitive%20Component%20Object%20Reference) (OtherBodyIndex :type Integer) (bFromSweep :type Boolean) (SweepResult :type Hit%20Result%20Structure%20%28by%20ref%29))
  (bind _asbp_base_character (Utilities|Casting|CastToBP_BaseCharacter OtherActor))
  (if (GameplayTags|HasTag (Variables|/Game/Maze/Core/Characterts/BP_BaseCharacter.BP_BaseCharacter_C|GetGameplayTags _asbp_base_character) "(TagName=\"Status.Charactet.Player.CurrentPlayer\")" true)
    (CallFunction|SetIsCompleted true)
    (Variables|/Script/Engine.PrimitiveComponent|SetbGenerateOverlapEvents (Variables|Default|GetBox) false)
    (Rendering|SetVisibility (Variables|Default|GetCube) false false)))

(event EventBeginPlay
  (|CallParentFunction)
  (if (not (CallFunction|GetIsActive))
    (Variables|/Script/Engine.PrimitiveComponent|SetbGenerateOverlapEvents (Variables|Default|GetBox) false)
    (Rendering|SetVisibility (Variables|Default|GetCube) false false)))

(event EventActivateQuest
  (|CallParentFunction)
  (Variables|/Script/Engine.PrimitiveComponent|SetbGenerateOverlapEvents (Variables|Default|GetBox) true)
  (Rendering|SetVisibility (Variables|Default|GetCube) true false))

(fn ConstructionScript
  (|CallParentFunction))